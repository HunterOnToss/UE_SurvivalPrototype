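; RPG stats Blueprint that tracks a character's experience and level.
; ChangeExperience adds experience, then checks it against ExperienceForNextLevel.
; Reaching the threshold adds one level, calls NextLevel and resets Experience from a calculation function, while the threshold itself stays unchanged here.
; Tick prints level, experience and threshold on screen every frame as a debug readout.
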(event EventBeginPlay)

(event EventTick
  (params (DeltaSeconds :type Float%20%28single-precision%29))
  (CallFunction|PrintRPGStats))

(fn ChangeExperience
  (params (ExperienceValue :type Float%20%28single-precision%29))
  (Variables|Default|SetExperience (+ ExperienceValue (Variables|Default|GetExperience)))
  (CallFunction|CheckExperienceforLevel))

(fn ChangeLevel
  (params (AddLevel :type Integer))
  (Variables|Default|SetLevel (+ AddLevel (Variables|Default|GetLevel))))

(fn CheckExperienceforLevel
  (if (>= (Variables|Default|GetExperience) (Variables|Default|GetExperienceForNextLevel))
    (CallFunction|ChangeLevel 1)
    (Default|CallNextLevel)
    (Variables|Default|SetExperience (CallFunction|CalculateExperienceforCurrentLevel))))

(fn CalculateExperienceforCurrentLevel
  (return (|({67DAF588-4D66-1740-E348-0FBC29627B2B}+({64B5039A-4BD1-E638-7B43-BA97F2580D3C}*100)))))

(fn PrintRPGStats
  (Development|PrintString (Utilities|String|Append "Level:" (Utilities|String|ToString(Integer) (Variables|Default|GetLevel))) true true "(R=0.000000,G=0.000000,B=0.000000,A=1.000000)" 0.0)
  (Development|PrintString (Utilities|String|Append "Experience:" (Utilities|String|ToString(Float) (Variables|Default|GetExperience))) true true "(R=1.000000,G=1.000000,B=1.000000,A=1.000000)" 0.0)
  (Development|PrintString (Utilities|String|Append "Experience to next level:" (Utilities|String|ToString(Float) (Variables|Default|GetExperienceForNextLevel))) true true "(R=1.000000,G=1.000000,B=1.000000,A=1.000000)" 0.0))